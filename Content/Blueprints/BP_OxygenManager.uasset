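; BP_OxygenManager is a manager actor that maintains the room connection graph between BP_OxygenArea actors.
; When its Update flag is set, the construction script caches every oxygen area in AllOxygenAreas and then clears the flag while processing them.
; It makes each ConnectedRooms link two-way and removes invalid entries, which a comment credits with fixing a major frame rate issue.
; The event graph has no runtime logic.
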(event EventBeginPlay)

(event Collision|EventActorBeginOverlap
  (params (OtherActor :type Actor%20Object%20Reference)))

(event EventTick
  (params (DeltaSeconds :type Float%20%28single-precision%29)))

(fn ConstructionScript
  (if (Variables|Default|GetUpdate)
    (bind _outactors (Actor|GetAllActorsOfClass "/Game/Blueprints/BP_OxygenArea.BP_OxygenArea_C"))
    (bind _output_get (Variables|Default|SetAll%20Oxygen%20Areas _outactors))
    ;[1 1 1] Fixes major frame rate issue caused by empty entries in the array
    (for _array_element _output_get
      (for _array_element_2 (Variables|/Game/Blueprints/BP_OxygenArea.BP_OxygenArea_C|GetConnected%20Rooms _array_element)
        (Utilities|IsValid _array_element_2
          (:Is%20Valid
            (if (not (Utilities|Array|ContainsItem (Variables|/Game/Blueprints/BP_OxygenArea.BP_OxygenArea_C|GetConnected%20Rooms _array_element_2) _array_element))
              (Utilities|Array|Add (Variables|/Game/Blueprints/BP_OxygenArea.BP_OxygenArea_C|GetConnected%20Rooms _array_element_2) _array_element)))
          (:Is%20Not%20Valid
            (Utilities|Array|RemoveItem (Variables|/Game/Blueprints/BP_OxygenArea.BP_OxygenArea_C|GetConnected%20Rooms _array_element) _array_element_2))))
      (Variables|Default|SetUpdate false))))