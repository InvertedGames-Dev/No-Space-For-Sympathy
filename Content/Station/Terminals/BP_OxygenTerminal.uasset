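; Station oxygen terminal that periodically supplies oxygen to every room while it is functional.
; A looping timer starts on BeginPlay, firing every second when functional and every minute otherwise.
; Each firing gives OxygenRefill to all of the station manager's rooms, or only prints the Functional state when broken.
; Repaired calls UpdateTimer, which restarts the timer at the rate matching the current state.
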(event Custom|Fill/Deflate%20Room
  (bind _functional (Variables|Default|GetFunctional))
  ;[1 1 1] Send info to are every minute/second
  (if _functional
    (for _array_element (Variables|/Game/Station/Blueprints/BP_StationManager.BP_StationManager_C|GetAll%20Station%20Rooms (Variables|Default|GetStationManagerReference))
      (Default|GiveOxygen _array_element (Variables|Default|GetOxygenRefill)))
    (else
      (Development|PrintString (Utilities|String|ToString(Boolean) _functional) true true "(R=0.000000,G=0.660000,B=1.000000,A=1.000000)" 0.0))))

(event Custom|Update%20Timer
  (Utilities|Time|ClearandInvalidateTimerbyHandle (stale _returnvalue))
  (bind _returnvalue (Utilities|Time|SetTimerbyEvent (delegate Custom|Fill/Deflate%20Room) (select (Variables|Default|GetFunctional) 1.0 6e+01) true)))

(event EventBeginPlay
  (|CallParentFunction)
  (bind _returnvalue (Utilities|Time|SetTimerbyEvent (delegate Custom|Fill/Deflate%20Room) (select (Variables|Default|GetFunctional) 1.0 6e+01) true)))

(event Collision|EventActorBeginOverlap
  (params (OtherActor :type Actor%20Object%20Reference))
  (|CallParentFunction OtherActor) ; This node is disabled and will not be called.\nDrag off pins to build functionality.
)

(event EventTick
  (params (DeltaSeconds :type Float%20%28single-precision%29))
  (|CallParentFunction DeltaSeconds) ; This node is disabled and will not be called.\nDrag off pins to build functionality.
)

(event EventRepaired
  (CallFunction|UpdateTimer))

(fn ConstructionScript
  (|CallParentFunction))