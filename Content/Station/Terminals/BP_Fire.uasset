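; BP_Fire is a station fire hazard that damages what it touches and consumes room oxygen until extinguished.
; A looping timer fires Burn every tenth of a second, damaging all actors overlapping its sphere and calling TakeOxygen on overlapping BP_MasterStationRoom actors.
; The Action event records a SpaceTrogladyte as Operator; an Extinguish action ends repair after a short delay and destroys the fire.
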(event Custom|Burn
  (for _array_element (Collision|GetOverlappingActors (Variables|Default|GetSphere) "/Script/Engine.Actor" :!class /Script/Engine.PrimitiveComponent)
    (Game|Damage|ApplyDamage _array_element 1.0 0 0)
    (bind _asbp_master_station_room (Utilities|Casting|CastToBP_MasterStationRoom _array_element))
    (Default|TakeOxygen _asbp_master_station_room 0 5.0))
  (Rendering|SetVisibility (Variables|Default|GetBrokenEffect) true false))

(event EventBeginPlay
  (|CallParentFunction)
  (Utilities|Time|SetTimerbyEvent (delegate Custom|Burn) 0.1 true)
  (Rendering|SetVisibility (Variables|Default|GetBrokenEffect) true false))

(event Collision|EventActorBeginOverlap
  (params (OtherActor :type Actor%20Object%20Reference))
  (|CallParentFunction OtherActor) ; This node is disabled and will not be called.\nDrag off pins to build functionality.
)

(event EventTick
  (params (DeltaSeconds :type Float%20%28single-precision%29))
  (|CallParentFunction DeltaSeconds) ; This node is disabled and will not be called.\nDrag off pins to build functionality.
)

(event EventAction
  (params (Action :type e_Actions%20Enum :default "NewEnumerator4") (Actor :type Actor%20Object%20Reference))
  ;[1 1 1] Action
  (CallFunction|EndAction "NewEnumerator4")
  (bind _asspace_trogladyte (Utilities|Casting|CastToSpaceTrogladyte Actor)
    (:then
      (Variables|Default|SetOperator _asspace_trogladyte))
    (:CastFailed
      _))
  (switch Utilities|FlowControl|Switch|Switchone_Actions Action
    (:NewEnumerator5
      (Utilities|FlowControl|Delay 2.0)
      (CallFunction|EndRepair)
      (Actor|DestroyActor))))

(fn ConstructionScript
  (|CallParentFunction))