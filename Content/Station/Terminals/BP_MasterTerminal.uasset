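; Base station terminal that a SpaceTrogladyte operator can repair or operate, with empty Operate, Open and Repaired events as hooks.
; Repair re-calls itself after a short delay, adding the operator's Skill to TerminalHealth and updating a progress bar widget until full or interrupted.
; UpdateActions derives the Functional flag, available Repair/Operate actions and broken-effect visibility from health.
; Self-selection opens a widget listing those actions.
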(event Custom|Repair
  (bind _progressbar (Variables|Default|GetProgressBar))
  ;[1 1 1] Repair
  (Audio|PlaySoundatLocation "/Game/Audio/SoundEffects/Hammer_Cue1.Hammer_Cue1" (Transformation|GetActorLocation) "0, 0, 0" 1.0 1.0 0.0 0 0 0)
  (if (Math|Boolean|ANDBoolean (< (Variables|Default|GetTerminalHealth) 1e+02) (Variables|Default|GetRepairing) (Utilities|IsValid (Variables|Default|GetOperator)))
    (Variables|Default|SetTerminalHealth (Math|Float|Clamp(Float) (+ (Variables|Default|GetTerminalHealth) (Math|Conversions|ToFloat(Integer) (Variables|/Game/NPCs/SpaceTrogladyte.SpaceTrogladyte_C|GetSkill (Variables|Default|GetOperator)))) 0.0 1e+02))
    (Utilities|IsValid _progressbar
      (:Is%20Valid
        (Default|UpdateProgress _progressbar (/ (Variables|Default|GetTerminalHealth) 1e+02)))
      (:Is%20Not%20Valid
        _))
    (Utilities|FlowControl|Delay 0.5)
    (CallFunction|Repair)
    (else
      (CallFunction|EndRepair))))

(event Custom|EndRepair
  (bind _operator (Variables|Default|GetOperator))
  (bind _progressbar (Variables|Default|GetProgressBar))
  ;[1 1 1] Repair
  (Utilities|IsValid _operator
    (:Is%20Valid
      (Default|EndAction _operator "NewEnumerator0"))
    (:Is%20Not%20Valid
      _))
  (Utilities|IsValid _progressbar
    (:Is%20Valid
      (Default|Close _progressbar))
    (:Is%20Not%20Valid
      _))
  (CallFunction|UpdateActions)
  (CallFunction|Repaired)
  (Variables|Default|SetRepairing false))

(event Custom|Open
  ;[1 1 1] Action
)

(event Custom|Operate
  ;[1 1 1] Action
)

(event Custom|Repaired
  ;[1 1 1] Action
)

(event EventBeginPlay
  ;[1 1 1] BeginPlay
  (bind _outactors (Actor|GetAllActorsOfClass "/Game/PlayerController/MasterPlayer.MasterPlayer_C"))
  (Variables|Default|SetPlayer (Utilities|Array|Get(acopy) _outactors))
  (CallFunction|UpdateActions)
  (bind _outactors_2 (Actor|GetAllActorsOfClass "/Game/Station/Blueprints/BP_StationManager.BP_StationManager_C"))
  (Variables|Default|SetStationManagerReference (Utilities|Array|Get(acopy) _outactors_2)))

(event EventSelfSelAction
  (params (Actor :type Actor%20Object%20Reference))
  ;[1 1 1] Self Sel Actions
  (bind _returnvalue (UserInterface|CreateWidget "/Game/UI/UI_SelfSelectedAction.UI_SelfSelectedAction_C" 0 (Transformation|GetActorLocation) (Variables|Default|GetActions) Actor self))
  (UserInterface|Viewport|AddtoViewport _returnvalue 0))

(event EventTick
  (params (DeltaSeconds :type Float%20%28single-precision%29)))

(event EventAlt-Selection)

(event EventAction
  (params (Action :type e_Actions%20Enum :default "NewEnumerator4") (Actor :type Actor%20Object%20Reference))
  ;[1 1 1] Action
  (CallFunction|EndAction "NewEnumerator4")
  (bind _asspace_trogladyte (Utilities|Casting|CastToSpaceTrogladyte Actor))
  (Variables|Default|SetOperator _asspace_trogladyte)
  (switch Utilities|FlowControl|Switch|Switchone_Actions Action
    (:NewEnumerator0
      (Variables|Default|SetRepairing true)
      (CallFunction|Repair)
      (bind _returnvalue (UserInterface|CreateWidget "/Game/UI/UI_ActionProgressBar.UI_ActionProgressBar_C" 0 (Transformation|GetActorLocation) (Utilities|Struct|MakeLinearColor 0.1 1.0 0.1 1.0) (Utilities|Text|ToText(String) (Utilities|String|EnumtoString Action))))
      (Variables|Default|SetProgressBar _returnvalue)
      (UserInterface|Viewport|AddtoViewport _returnvalue 0))
    (:NewEnumerator1
      (CallFunction|Operate))
    (:NewEnumerator3
      (CallFunction|Open))))

(event EventEndAction
  (params (Action :type e_Actions%20Enum :default "NewEnumerator4") (Actor :type Actor%20Object%20Reference))
  ;[1 1 1] EndAction
  (CallFunction|EndRepair)
  (Variables|Default|SetOperator 0)
  (Variables|Default|SetRepairing false))

(event Collision|EventActorBeginOverlap
  (params (OtherActor :type Actor%20Object%20Reference)))

(fn ConstructionScript)

(fn UpdateActions
  (bind _actions (Variables|Default|GetActions))
  (bind _actions_2 (Variables|Default|GetActions))
  (bind _returnvalue (Utilities|Array|ContainsItem _actions_2 "NewEnumerator0"))
  (Utilities|FlowControl|Sequence
    (:then_0
      (Variables|Default|SetFunctional (not (< (Variables|Default|GetTerminalHealth) 9e+01)))
      (if (== (Variables|Default|GetTerminalHealth) 1e+02)
        (if _returnvalue
          (Utilities|Array|RemoveItem _actions "NewEnumerator0"))
        (if (not (Utilities|Array|ContainsItem _actions "NewEnumerator1")) :!label _label
          (Utilities|Array|Add _actions "NewEnumerator1"))
        (else
          (if _returnvalue
            _
            (else
              (Utilities|Array|Add _actions_2 "NewEnumerator0")))
          (if (< (Variables|Default|GetTerminalHealth) 9e+01)
            (Utilities|Array|RemoveItem _actions_2 "NewEnumerator1")
            (else
              (goto _label))))))
    (:then_1
      (Rendering|SetVisibility (Variables|Default|GetBrokenEffect) (Utilities|Array|ContainsItem (Variables|Default|GetActions) "NewEnumerator0") false))))