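; BP_BasicRoom1 is a station room Blueprint with toggleable wall and window segments.
; Its construction script passes three wall flags to GenerateWall, one each for two wall segments and a window segment.
; GenerateWall sets a segment's visibility and matches its collision, enabling query and physics when shown and disabling collision when hidden.
; The event graph holds only disabled placeholder events, so the Blueprint adds no runtime logic.
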(event EventBeginPlay
  (|CallParentFunction) ; This node is disabled and will not be called.\nDrag off pins to build functionality.
)

(event Collision|EventActorBeginOverlap
  (params (OtherActor :type Actor%20Object%20Reference)))

(event EventTick
  (params (DeltaSeconds :type Float%20%28single-precision%29))
  (|CallParentFunction DeltaSeconds) ; This node is disabled and will not be called.\nDrag off pins to build functionality.
)

(fn ConstructionScript
  (Utilities|GenerateWall (Variables|Default|GetWall1) (Variables|Default|GetWallSegment))
  (Utilities|GenerateWall (Variables|Default|GetWall2) (Variables|Default|GetWindowSegment))
  (Utilities|GenerateWall (Variables|Default|GetWall3) (Variables|Default|GetWallSegment1))
  (|CallParentFunction))