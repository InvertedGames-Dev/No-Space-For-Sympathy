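; BP_Corridor1 is a station corridor room with its own oxygen store and two configurable door slots.
; The construction script feeds the Door1 and Door2 flags through a shared helper that selects the child actor class, placing BP_Door when a flag is set.
; BeginPlay runs the parent logic, then sets oxygen capacity and level to the same starting value, so the corridor begins full.
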(event EventBeginPlay
  (|CallParentFunction)
  (Variables|Default|SetOxygen%20Capacity 5e+02)
  (Variables|Default|SetOxygen%20Level 5e+02))

(event Collision|EventActorBeginOverlap
  (params (OtherActor :type Actor%20Object%20Reference)))

(event EventTick
  (params (DeltaSeconds :type Float%20%28single-precision%29))
  (|CallParentFunction DeltaSeconds) ; This node is disabled and will not be called.\nDrag off pins to build functionality.
)

(fn ConstructionScript
  (Utilities|Ye (Variables|Default|GetChildActor1) (Variables|Default|GetDoor1))
  (Utilities|Ye (Variables|Default|GetChildActor) (Variables|Default|GetDoor2))
  (|CallParentFunction))