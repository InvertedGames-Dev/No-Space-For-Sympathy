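; Station room actor that simulates its own oxygen supply, drained by the actors inside its box volume and printed on screen each tick.
; A looping one-second timer deducts oxygen per overlapping breather and sends a kill message once the level is empty.
; A faster timer pulls oxygen from connected rooms with higher fill ratios to equalize them.
; The construction script sizes the volume and makes room connections two-way through BP_StationManager's room list.
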(event OnComponentBeginOverlap(OxygenArea)
  (params (OverlappedComponent :type Primitive%20Component%20Object%20Reference) (OtherActor :type Actor%20Object%20Reference) (OtherComp :type Primitive%20Component%20Object%20Reference) (OtherBodyIndex :type Integer) (bFromSweep :type Boolean) (SweepResult :type Hit%20Result%20Structure%20%28by%20ref%29))
  ;[1 1 1] Adding npcs to the room
  (Utilities|Array|Add (Variables|Default|GetOxygen%20Breathers) OtherActor))

(event OnComponentEndOverlap(OxygenArea)
  (params (OverlappedComponent :type Primitive%20Component%20Object%20Reference) (OtherActor :type Actor%20Object%20Reference) (OtherComp :type Primitive%20Component%20Object%20Reference) (OtherBodyIndex :type Integer))
  ;[1 1 1] Adding npcs to the room
  (Utilities|Array|RemoveItem (Variables|Default|GetOxygen%20Breathers) OtherActor))

(event Custom|Calculate%20Oxygen
  ;[1 1 1] Calculate oxygen breathers
  (for _array_element (Variables|Default|GetOxygen%20Breathers)
    (Class|BPIOxygen|GetOxygenUsage(Message) _array_element self)
    (if (== (Variables|Default|GetOxygen%20Level) 0.0)
      (Class|BPIOxygen|Kill(Message) self)
      (else
        (Variables|Default|SetOxygen%20Level (Math|Float|Clamp(Float) (- (Variables|Default|GetOxygen%20Level) 1.0) 0.0 (Variables|Default|GetOxygen%20Capacity)))))))

(event Custom|Take%20Oxygen
  (params (Room :type BP%20Station%20Room%20Object%20Reference) (Oxygen :type Float%20%28single-precision%29))
  ;[1 1 1] Moving oxygen between rooms
  (Variables|Default|SetOxygen%20Level (- (Variables|Default|GetOxygen%20Level) Oxygen))
  (CallFunction|GiveOxygen Room Oxygen))

(event Custom|Give%20Oxygen
  (params (Oxygen :type Float%20%28single-precision%29))
  ;[1 1 1] Moving oxygen between rooms
  (Variables|Default|SetOxygen%20Level (+ Oxygen (Variables|Default|GetOxygen%20Level))))

(event Custom|Equalize%20oxygen%20levels%20with%20adjacent%20rooms
  (bind _connected_rooms (Variables|Default|GetConnected%20Rooms))
  ;[1 1 1] Equalize oxygen
  (if (Utilities|Array|IsValidIndex _connected_rooms)
    (for _array_element _connected_rooms
      (if (> (/ (Variables|BP_StationRoom_C|GetOxygen%20Level _array_element) (Variables|BP_StationRoom_C|GetOxygen%20Capacity _array_element)) (/ (Variables|Default|GetOxygen%20Level) (Variables|Default|GetOxygen%20Capacity)))
        (CallFunction|TakeOxygen _array_element self 1.0)))))

(event EventBeginPlay
  (Utilities|Time|SetTimerbyEvent (delegate Custom|Calculate%20Oxygen) 1.0 true)
  (Utilities|Time|SetTimerbyEvent (delegate Custom|Equalize%20oxygen%20levels%20with%20adjacent%20rooms) 0.02 true))

(event EventTick
  (params (DeltaSeconds :type Float%20%28single-precision%29))
  (Development|PrintString (Utilities|String|ToString(Text) (Utilities|Text|FormatText "{Room Name} Oxygen: {Oxygen Amount}" (Utilities|Text|ToText(String) (Variables|Default|GetRoom%20Name)) (Variables|Default|GetOxygen%20Level))) true true "(R=0.000000,G=1.000000,B=0.899574,A=1.000000)" DeltaSeconds))

(fn ConstructionScript
  (bind _self self)
  (Components|Box|SetBoxExtent (Variables|Default|GetOxygen%20Area) (Variables|Default|GetBox%20Extent) true)
  (bind _outactors (Actor|GetAllActorsOfClass "/Game/Station/Blueprints/BP_StationManager.BP_StationManager_C"))
  (bind _output_get (Variables|Default|SetOxygen%20Manager (Utilities|Array|Get(acopy) _outactors)))
  (for _array_element (Variables|Default|GetConnected%20Rooms)
    (if (not (Utilities|Array|ContainsItem (Variables|BP_StationRoom_C|GetConnected%20Rooms (Utilities|Array|Get(acopy) (Variables|/Game/Station/Blueprints/BP_StationManager.BP_StationManager_C|GetAll%20Station%20Rooms _output_get) (Utilities|Array|FindItem (Variables|/Game/Station/Blueprints/BP_StationManager.BP_StationManager_C|GetAll%20Station%20Rooms _output_get) _array_element))) _self))
      (Utilities|Array|Add (Variables|BP_StationRoom_C|GetConnected%20Rooms (Utilities|Array|Get(acopy) (Variables|/Game/Station/Blueprints/BP_StationManager.BP_StationManager_C|GetAll%20Station%20Rooms _output_get) (Utilities|Array|FindItem (Variables|/Game/Station/Blueprints/BP_StationManager.BP_StationManager_C|GetAll%20Station%20Rooms _output_get) _array_element))) _self))))