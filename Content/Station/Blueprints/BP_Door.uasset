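; Station sliding door, built on a parent with terminal health and broken state, that opens when an actor overlaps it unless broken.
; Both panels slide apart, hold for OpenTime via retriggerable delays, then slide closed.
; Opening starts a looping timer that gradually equalizes oxygen between Room1 and Room2 until cleared after closing.
; An entry is removed from Actions during the cycle and re-added afterward.
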(event Custom|Open2
  (bind _doorpanelright (Variables|Default|GetDoorPanelRight))
  (Components|MoveComponentTo _doorpanelright "0,-200.000000,0.000000" "0, 0, 0" true true 0.5 false)
  (Utilities|FlowControl|RetriggerableDelay (Variables|Default|GetOpenTime))
  (Components|MoveComponentTo _doorpanelright "0, 0, 0" "0, 0, 0" true true 0.5 false))

(event Custom|Vent
  (Utilities|IsValid (Variables|Default|GetRoom2)
    (:Is%20Valid
      (CallFunction|EqualizeOxygen (Variables|Default|GetRoom1) (Variables|Default|GetRoom2) 0.1))
    (:Is%20Not%20Valid
      (Development|PrintString "InvalidRoom"))))

(event EventBeginPlay
  (Variables|Default|SetTerminalHealth 1e+02)
  (|CallParentFunction))

(event Collision|EventActorBeginOverlap
  (params (OtherActor :type Actor%20Object%20Reference))
  (|CallParentFunction OtherActor)
  (CallFunction|Open))

(event EventTick
  (params (DeltaSeconds :type Float%20%28single-precision%29))
  (|CallParentFunction DeltaSeconds))

(event EventOpen
  (bind _doorpanelleft (Variables|Default|GetDoorPanelLeft))
  (Development|PrintString (Utilities|String|ToString(Float) (Variables|Default|GetTerminalHealth)))
  (if (not (CallFunction|IsBroken?))
    (bind _returnvalue (Utilities|Time|SetTimerbyEvent (delegate Custom|Vent) 0.5 true))
    (Utilities|Array|RemoveItem (Variables|Default|GetActions) "NewEnumerator3")
    (CallFunction|Open2)
    (Components|MoveComponentTo _doorpanelleft "0,200.000000,0.000000" "0, 0, 0" true true 0.5 false)
    (Utilities|FlowControl|RetriggerableDelay (Variables|Default|GetOpenTime))
    (Components|MoveComponentTo _doorpanelleft "0, 0, 0" "0, 0, 0" true true 0.5 false)
    (Utilities|Array|Add (Variables|Default|GetActions) "NewEnumerator3")
    (Utilities|Time|ClearandInvalidateTimerbyHandle _returnvalue)))

(fn ConstructionScript)